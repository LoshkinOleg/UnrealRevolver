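; Player pawn simulating a hand-manipulated six-shot revolver, with movement and yaw aiming.
; Enhanced Input axes drive hammer, trigger, safety, cylinder and ejector meshes, with state checks gating single- or double-action firing.
; Firing advances the chamber, then line-traces and spawns hit particles, or dry-fires on spent rounds.
; With the cylinder open, rounds move along splines via the ejector or randomised tilt-based sliding, spawning ejected-bullet actors until reloaded individually.
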(event `self.ReceiveBeginPlay`
  (for _ (range 6)
    (`KismetArrayLibrary.Array_Add` (`self.BulletPositions`))
    (`KismetArrayLibrary.Array_Add` (`self.BulletSlidingFactors`))
    (`KismetArrayLibrary.Array_Add` (`self.EjectedBullets`))
    (`KismetArrayLibrary.Array_Add` (`self.SpentBullets`)))
  (`KismetArrayLibrary.Array_Add` (`self.BulletMeshes`) (`self.Bullet0`))
  (`KismetArrayLibrary.Array_Add` (`self.BulletSplines`) (`self.Spline0`))
  (`KismetArrayLibrary.Array_Add` (`self.BulletMeshes`) (`self.Bullet1`))
  (`KismetArrayLibrary.Array_Add` (`self.BulletSplines`) (`self.Spline1`))
  (`KismetArrayLibrary.Array_Add` (`self.BulletMeshes`) (`self.Bullet2`))
  (`KismetArrayLibrary.Array_Add` (`self.BulletSplines`) (`self.Spline2`))
  (`KismetArrayLibrary.Array_Add` (`self.BulletMeshes`) (`self.Bullet3`))
  (`KismetArrayLibrary.Array_Add` (`self.BulletSplines`) (`self.Spline3`))
  (`KismetArrayLibrary.Array_Add` (`self.BulletMeshes`) (`self.Bullet4`))
  (`KismetArrayLibrary.Array_Add` (`self.BulletSplines`) (`self.Spline4`))
  (`KismetArrayLibrary.Array_Add` (`self.BulletMeshes`) (`self.Bullet5`))
  (`KismetArrayLibrary.Array_Add` (`self.BulletSplines`) (`self.Spline5`))
  (`self.PickNewSlidingFactors`)
  (`AudioComponent.Stop` (`self.Audio_Bang`))
  (`AudioComponent.Stop` (`self.Audio_Racket`))
  (`AudioComponent.Stop` (`self.Audio_Click`))
  (`AudioComponent.Stop` (`self.Audio_DryFire`)))

(event `self.ReceiveTick`
  (params (DeltaSeconds :type "Float (single-precision)"))
  (`self.UpdateBullets`))

(event `EnhancedInput|/Game/Blueprints/Inputs/Main/Input_CockHammer`
  (params (ActionValue :type "Float (double-precision)") (ElapsedSeconds :type "Float (double-precision)") (TriggeredSeconds :type "Float (double-precision)") (InputAction :type "InputAction Object Reference" :default "/Game/Blueprints/Inputs/Main/Input_CockHammer.Input_CockHammer"))
  (:`Triggered`
    (`self.ProcessHammerCocking` (`KismetMathLibrary.FClamp` ActionValue) :!label _label))
  (:`Completed`
    (goto _label)))

(event `EnhancedInput|/Game/Blueprints/Inputs/Main/Input_PullTrigger`
  (params (ActionValue :type "Float (double-precision)") (ElapsedSeconds :type "Float (double-precision)") (TriggeredSeconds :type "Float (double-precision)") (InputAction :type "InputAction Object Reference" :default "/Game/Blueprints/Inputs/Main/Input_PullTrigger.Input_PullTrigger"))
  (:`Triggered`
    (`self.Process Trigger Pull` ActionValue :!label _label_2))
  (:`Completed`
    (goto _label_2)))

(event `EnhancedInput|/Game/Blueprints/Inputs/Main/Input_OpenCylinder`
  (params (ActionValue :type Boolean) (ElapsedSeconds :type "Float (double-precision)") (TriggeredSeconds :type "Float (double-precision)") (InputAction :type "InputAction Object Reference" :default "/Game/Blueprints/Inputs/Main/Input_OpenCylinder.Input_OpenCylinder"))
  (:`Started`
    (bind _isa (`/Engine/EditorBlueprintResources/StandardMacros.FlipFlop`)
      (:`A`
        _)
      (:`B`
        _))
    (`self.ProcessOpenCylinder` _isa)
    (`self.PickNewSlidingFactors`)))

(event `EnhancedInput|/Game/Blueprints/Inputs/Main/Input_SafetyOn`
  (params (ActionValue :type Boolean) (ElapsedSeconds :type "Float (double-precision)") (TriggeredSeconds :type "Float (double-precision)") (InputAction :type "InputAction Object Reference" :default "/Game/Blueprints/Inputs/Main/Input_SafetyOn.Input_SafetyOn"))
  (:`Triggered`
    (`self.ProcessSafety` true)))

(event `EnhancedInput|/Game/Blueprints/Inputs/Main/Input_SafetyOff`
  (params (ActionValue :type Boolean) (ElapsedSeconds :type "Float (double-precision)") (TriggeredSeconds :type "Float (double-precision)") (InputAction :type "InputAction Object Reference" :default "/Game/Blueprints/Inputs/Main/Input_SafetyOff.Input_SafetyOff"))
  (:`Triggered`
    (`self.ProcessSafety` false)))

(event `EnhancedInput|/Game/Blueprints/Inputs/Main/Input_TurnGun`
  (params (ActionValue :type "Vector2D Structure") (ElapsedSeconds :type "Float (double-precision)") (TriggeredSeconds :type "Float (double-precision)") (InputAction :type "InputAction Object Reference" :default "/Game/Blueprints/Inputs/Main/Input_TurnGun.Input_TurnGun"))
  (bind (_x _y) (`KismetMathLibrary.BreakVector2D` ActionValue))
  (:`Triggered`
    (`self.ProcessTurnGun` _x _y :!label _label_3))
  (:`Completed`
    (goto _label_3)))

(event `EnhancedInput|/Game/Blueprints/Inputs/Main/Input_EjectShells`
  (params (ActionValue :type "Float (double-precision)") (ElapsedSeconds :type "Float (double-precision)") (TriggeredSeconds :type "Float (double-precision)") (InputAction :type "InputAction Object Reference" :default "/Game/Blueprints/Inputs/Main/Input_EjectShells.Input_EjectShells"))
  (:`Triggered`
    (`self.ProcessEjectShells` ActionValue :!label _label_4))
  (:`Completed`
    (goto _label_4)))

(event `EnhancedInput|/Game/Blueprints/Inputs/Main/Input_LoadBullet`
  (params (ActionValue :type Boolean) (ElapsedSeconds :type "Float (double-precision)") (TriggeredSeconds :type "Float (double-precision)") (InputAction :type "InputAction Object Reference" :default "/Game/Blueprints/Inputs/Main/Input_LoadBullet.Input_LoadBullet"))
  (:`Started`
    (`self.LoadNextBullet`)))

(event `EnhancedInput|/Game/Blueprints/Inputs/Main/Input_Move`
  (params (ActionValue :type "Vector2D Structure") (ElapsedSeconds :type "Float (double-precision)") (TriggeredSeconds :type "Float (double-precision)") (InputAction :type "InputAction Object Reference" :default "/Game/Blueprints/Inputs/Main/Input_Move.Input_Move"))
  (bind (_x _y) (`KismetMathLibrary.BreakVector2D` ActionValue))
  (:`Triggered`
    (`self.ProcessMove` _x _y :!label _label_5))
  (:`Completed`
    (goto _label_5)))

(event `EnhancedInput|/Game/Blueprints/Inputs/Main/Input_Aim`
  (params (ActionValue :type "Vector2D Structure") (ElapsedSeconds :type "Float (double-precision)") (TriggeredSeconds :type "Float (double-precision)") (InputAction :type "InputAction Object Reference" :default "/Game/Blueprints/Inputs/Main/Input_Aim.Input_Aim"))
  (bind (_x _y) (`KismetMathLibrary.BreakVector2D` ActionValue))
  (:`Triggered`
    (`self.ProcessAim` _x _y :!label _label_6))
  (:`Completed`
    (goto _label_6)))

(event `EnhancedInput|/Game/Blueprints/Inputs/Main/Input_ResetGunOrientation`
  (params (ActionValue :type Boolean) (ElapsedSeconds :type "Float (double-precision)") (TriggeredSeconds :type "Float (double-precision)") (InputAction :type "InputAction Object Reference" :default "/Game/Blueprints/Inputs/Main/Input_ResetGunOrientation.Input_ResetGunOrientation"))
  (:`Completed`
    (`self.ProcessResetGunOrientation`)))

(fn `CanCockHammer`
  (returns (CanCockHammer :type Boolean))
  (return (not (`self.SafetyAxis`))))

(fn `CanFire`
  (returns (CanFire :type Boolean))
  (bind _fullycocked (`self.IsHammerCocked`))
  (return (and _fullycocked (not (`self.SafetyAxis`)) (not (`self.CylinderRadialAxis`)) (not (`self.Firing`)))))

(fn `CanPullTrigger`
  (returns (CanPullTrigger :type Boolean))
  (return (not (`self.SafetyAxis`))))

(fn `FireGun`
  (bind _returnvalue (`SceneComponent.K2_GetComponentLocation` (`self.revolver_body`)))
  (set `self.Firing` true)
  (bind _output_get (set `self.HammerAxis` 0.0))
  (`self.SetHammerRotation` _output_get)
  (bind _result (`/Engine/EditorBlueprintResources/StandardMacros.IncrementInt` (`self.CurrentBullet`))
    (:`  `
      (set `self.CurrentBullet` (mod _result 6))
      (if (not (`|GetArrayItem` (`self.SpentBullets`) (`self.CurrentBullet`)))
        (`AudioComponent.Play` (`self.Audio_Bang`) 0.0)
        (`KismetArrayLibrary.Array_Set` (`self.SpentBullets`) (`self.CurrentBullet`) true)
        (bind _outhit (`KismetSystemLibrary.LineTraceSingle` :`Start` _returnvalue :`End` (+ _returnvalue (* (`KismetMathLibrary.NegateVector` (`SceneComponent.GetForwardVector` (`self.revolver_body`))) 10000.0)) :`TraceChannel` "TraceTypeQuery1" :`DrawDebugType` "ForOneFrame"))
        (bind (_bblockinghit _binitialoverlap _time _distance _location) (`GameplayStatics.BreakHitResult` _outhit))
        (if _bblockinghit
          (`KismetSystemLibrary.PrintString` "Hello")
          (`|SpawnActorFromClass` "/Game/Blueprints/HitParticles.HitParticles_C" (`KismetMathLibrary.Conv_VectorToTransform` _location) "AlwaysSpawn" "OverrideRootScale" null null))
        (else
          (`AudioComponent.Play` (`self.Audio_DryFire`) 0.0))))))

(fn `IsEjectorDepressed`
  (returns (FullyDepressed :type Boolean))
  (return (`KismetMathLibrary.NearlyEqual_FloatFloat` (`self.EjectorAxis`) 1.0 0.05)))

(fn `IsHammerAtRest`
  (returns (Released :type Boolean))
  (return (`KismetMathLibrary.NearlyEqual_FloatFloat` (`self.HammerAxis`) 0.0 0.05)))

(fn `IsHammerCocked`
  (returns (FullyCocked :type Boolean))
  (return (> (`self.HammerAxis`) 0.9)))

(fn `IsTriggerAtRest`
  (returns (Released :type Boolean))
  (return (`KismetMathLibrary.NearlyEqual_FloatFloat` (`self.TriggerAxis`) 0.0 0.05)))

(fn `IsTriggerPulled`
  (returns (FullyPulled :type Boolean))
  (return (> (`self.TriggerAxis`) 0.9)))

(fn `LoadNextBullet`
  (if (`self.CylinderRadialAxis`)
    (bind _result (`/Engine/EditorBlueprintResources/StandardMacros.IncrementInt` (`self.CurrentBullet`))
      (:`  `
        (set `self.CurrentBullet` (mod _result 6))
        (`KismetArrayLibrary.Array_Set` (`self.EjectedBullets`) (`self.CurrentBullet`))
        (`SceneComponent.SetVisibility` (`|GetArrayItem` (`self.BulletMeshes`) (`self.CurrentBullet`)) true false)
        (`KismetArrayLibrary.Array_Set` (`self.BulletPositions`) (`self.CurrentBullet`))
        (`KismetArrayLibrary.Array_Set` (`self.SpentBullets`) (`self.CurrentBullet`))))))

(fn `PickNewSlidingFactors`
  (for (_ _array_index) (`self.BulletSlidingFactors`)
    (`KismetArrayLibrary.Array_Set` (`self.BulletSlidingFactors`) _array_index (`KismetMathLibrary.RandomFloatInRange` (`self.kBulletSlidingFactorRangeMin_`) (`self.kBulletSlidingFactorRangeMax_`)))))

(fn `Process Trigger Pull`
  (params (PullingAxis :type "Float (double-precision)"))
  (if (not (`self.SafetyAxis`))
    (if (and (< (`self.TriggerAxis`) 0.5) (> (`local.PullingAxis`) 0.5))
      (`AudioComponent.Play` (`self.Audio_Racket`) 0.0))
    (bind _output_get (set `self.TriggerAxis` (`local.PullingAxis`)))
    (`self.SetTriggerRotation` _output_get)
    (if (not (`self.Firing`))
      (bind _fullycocked (`self.IsHammerCocked`))
      (if _fullycocked
        (bind _canfire (`self.CanFire`))
        (if _canfire
          (`self.FireGun`))
        (else
          (bind _output_get_2 (set `self.HammerAxis` (`local.PullingAxis`)))
          (`self.SetHammerRotation` _output_get_2)
          (bind _canfire_2 (`self.CanFire`))
          (if _canfire_2
            (`self.FireGun`))))
      (else
        (bind _released (`self.IsTriggerAtRest`))
        (if (and _released (`self.Firing`))
          (set `self.Firing` false))))))

(fn `ProcessAim`
  (params (X :type "Float (double-precision)") (Y :type "Float (double-precision)"))
  (`SceneComponent.K2_AddWorldRotation` (`self.DefaultSceneRoot`) (`KismetMathLibrary.MakeRotator` 0.0 0.0 (* (`KismetMathLibrary.MultiplyMultiply_FloatFloat` (`local.X`) 3.0) 3.0)) false false))

(fn `ProcessEjectShells`
  (params (EjectionAxis :type "Float (double-precision)"))
  (set `self.EjectorAxis` EjectionAxis)
  (if (`self.CylinderRadialAxis`)
    (`self.SetEjectorPosition` (`local.EjectionAxis`))
    (else
      (`self.SetEjectorPosition` 0.0))))

(fn `ProcessHammerCocking`
  (params (CockingAxis :type "Float (double-precision)"))
  (if (not (`self.SafetyAxis`))
    (if (and (< (`self.HammerAxis`) 0.5) (> (`local.CockingAxis`) 0.5))
      (`AudioComponent.Play` (`self.Audio_Racket`) 0.0))
    (bind _fullycocked (`self.IsHammerCocked`))
    (if (not _fullycocked)
      (bind _output_get (set `self.HammerAxis` (`local.CockingAxis`)))
      (`self.SetHammerRotation` _output_get)
      (else
        (bind _fullypulled (`self.IsTriggerPulled`))
        (if _fullypulled
          (bind _output_get_2 (set `self.HammerAxis` (`local.CockingAxis`)))
          (`self.SetHammerRotation` _output_get_2))))))

(fn `ProcessMove`
  (params (X :type "Float (double-precision)") (Y :type "Float (double-precision)"))
  (`self.K2_SetActorLocation` (+ (`self.K2_GetActorLocation`) (* (`local.X`) 10.0 (`self.GetActorRightVector`)) (* (`local.Y`) 10.0 (`self.GetActorForwardVector`))) true))

(fn `ProcessOpenCylinder`
  (params (InputValue :type Boolean))
  (if (not (`local.InputValue`))
    (set `self.CurrentBullet` 0))
  (bind _fullycocked (`self.IsHammerCocked`))
  (if (not _fullycocked)
    (bind _output_get (set `self.CylinderRadialAxis` (`local.InputValue`)))
    (`self.SetCylinderRotation` _output_get)))

(fn `ProcessResetGunOrientation`
  (`SceneComponent.K2_SetRelativeRotation` (`self.revolver_body`) (struct :`Yaw` 180.0) false false))

(fn `ProcessSafety`
  (params (InputValue :type Boolean))
  (bind _fullycocked (`self.IsHammerCocked`))
  (if (not _fullycocked)
    (bind _fullypulled (`self.IsTriggerPulled`))
    (if (not _fullypulled)
      (bind _output_get (set `self.SafetyAxis` (`local.InputValue`)))
      (`self.SetSafetyPosition` _output_get))))

(fn `ProcessTurnGun`
  (params (X :type "Float (double-precision)") (Y :type "Float (double-precision)"))
  (`SceneComponent.K2_AddRelativeRotation` (`self.revolver_body`) (`KismetMathLibrary.MakeRotator` 0.0 (- 0.0 (`local.Y`)) (`local.X`)) false false))

(fn `SetBulletPosition`
  (params (Idx :type Integer))
  (`SceneComponent.K2_SetRelativeLocation` (`|GetArrayItem` (`self.BulletMeshes`) (`local.Idx`)) (`SplineComponent.GetLocationAtTime` (`|GetArrayItem` (`self.BulletSplines`) (`local.Idx`)) (`|GetArrayItem` (`self.BulletPositions`) (`local.Idx`)) "Local" false) false true))

(fn `SetCylinderRotation`
  (params (OpenOrClosed :type Boolean))
  (locals (Value :type "Float (double-precision)"))
  (if OpenOrClosed
    (`SceneComponent.K2_SetRelativeRotation` (`self.revolver_cylinder`) (struct :`Roll` 90.0) false false)
    (else
      (`SceneComponent.K2_SetRelativeRotation` :`self` (`self.revolver_cylinder`)))))

(fn `SetEjectorPosition`
  (params (Percentage :type "Float (double-precision)"))
  (`SceneComponent.K2_SetRelativeLocation` (`self.revolver_ejector`) (`KismetMathLibrary.VLerp` (21.3 0.0 42.6) (31.3 0.0 42.6) Percentage) false true))

(fn `SetHammerRotation`
  (params (Percentage :type "Float (double-precision)"))
  (locals (Value :type "Float (double-precision)"))
  (set `local.Value` Percentage)
  (if (not (not (`KismetMathLibrary.NearlyEqual_FloatFloat` (`local.Value`) 0.0 0.05)))
    (set `local.Value` 0.0))
  (if (not (not (> (`local.Value`) 0.9)))
    (set `local.Value` 1.0))
  (`SceneComponent.K2_SetRelativeRotation` (`self.revolver_hammer`) (`KismetMathLibrary.MakeRotator` 0.0 (* (`local.Value`) -65.0)) false false))

(fn `SetSafetyPosition`
  (params (OnOrOff :type Boolean))
  (locals (Value :type "Float (double-precision)"))
  (if OnOrOff
    (`SceneComponent.K2_SetRelativeLocation` (`self.revolver_safety`) (80.0 27.0 34.0) false true)
    (else
      (`SceneComponent.K2_SetRelativeLocation` (`self.revolver_safety`) (63.0 27.0 34.0) false true))))

(fn `SetTriggerRotation`
  (params (Percentage :type "Float (double-precision)"))
  (locals (Value :type "Float (double-precision)"))
  (set `local.Value` Percentage)
  (if (not (not (`KismetMathLibrary.NearlyEqual_FloatFloat` (`local.Value`) 0.0 0.05)))
    (set `local.Value` 0.0))
  (if (not (not (> (`local.Value`) 0.9)))
    (set `local.Value` 1.0))
  (`SceneComponent.K2_SetRelativeRotation` (`self.revolver_trigger`) (`KismetMathLibrary.MakeRotator` 0.0 (* (`local.Value`) 54.0)) false false))

(fn `UpdateBullets`
  (if (`self.CylinderRadialAxis`)
    (for (_ _array_index) (`self.BulletPositions`)
      (`self.UpdateSingleBullet` _array_index))
    (else
      (for (_ _array_index_2) (`self.BulletPositions`)
        (`KismetArrayLibrary.Array_Set` (`self.BulletPositions`) _array_index_2)
        (`self.SetBulletPosition` _array_index_2)))))

(fn `UpdateSingleBullet`
  (params (Idx :type Integer))
  (if (<= (`|GetArrayItem` (`self.BulletPositions`) (`local.Idx`)) (* (`self.EjectorAxis`) (`self.kBulletEjectionOffset_`)))
    (`KismetArrayLibrary.Array_Set` (`self.BulletPositions`) (`local.Idx`) (`KismetMathLibrary.FClamp` (* (`self.EjectorAxis`) (`self.kBulletEjectionOffset_`))))
    (elif (> (`KismetMathLibrary.Abs` (* (`self.ComputeDotBetweenFrontAndUp`) (`|GetArrayItem` (`self.BulletSlidingFactors`) (`local.Idx`)))) (`self.kBulletSlidingThreshold_`))
      (`KismetArrayLibrary.Array_Set` (`self.BulletPositions`) (`local.Idx`) (`KismetMathLibrary.FClamp` (+ (`|GetArrayItem` (`self.BulletPositions`) (`local.Idx`)) (* (`self.ComputeDotBetweenFrontAndUp`) (`|GetArrayItem` (`self.BulletSlidingFactors`) (`local.Idx`))))))))
  (if (and (not (`|GetArrayItem` (`self.EjectedBullets`) (`local.Idx`))) (`KismetMathLibrary.NearlyEqual_FloatFloat` (`|GetArrayItem` (`self.BulletPositions`) (`local.Idx`)) 1.0 0.075))
    (`SceneComponent.SetVisibility` (`|GetArrayItem` (`self.BulletMeshes`) (`local.Idx`)) false false)
    (`|SpawnActorFromClass` "/Game/Blueprints/EjectedBullet.EjectedBullet_C" (`SceneComponent.K2_GetComponentToWorld` (`|GetArrayItem` (`self.BulletMeshes`) (`local.Idx`))) "AdjustIfPossibleButAlwaysSpawn" "OverrideRootScale" null null)
    (`KismetArrayLibrary.Array_Set` (`self.EjectedBullets`) (`local.Idx`) true))
  (`self.SetBulletPosition` (`local.Idx`)))

(fn `UserConstructionScript`)