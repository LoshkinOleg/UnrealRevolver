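; Bullet Blueprint that slides a static mesh along a spline while it is active.
; Each tick it advances a normalized spline position by Mass times the dot product of the constant forward vector and the spline's up vector, so the spline's orientation sets direction and speed.
; The position is clamped to the spline's ends and applied as a teleporting relative move, with no delta-time scaling.
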(event `self.ReceiveTick`
  (params (DeltaSeconds :type "Float (single-precision)"))
  (`self.UpdatePosAlongSpline`))

(fn `UpdatePosAlongSpline`
  (if (`self.Active`)
    (set `self.PosAlongSpline` (`KismetMathLibrary.FClamp` (+ (`self.PosAlongSpline`) (* (`self.Mass`) (`KismetMathLibrary.Dot_VectorVector` (`KismetMathLibrary.Vector_Forward`) (`SceneComponent.GetUpVector` (`self.Spline`)))))))
    (`SceneComponent.K2_SetRelativeLocation` (`self.StaticMesh`) (`SplineComponent.GetLocationAtTime` (`self.Spline`) (`self.PosAlongSpline`) "Local" false) false true)))

(fn `UserConstructionScript`)