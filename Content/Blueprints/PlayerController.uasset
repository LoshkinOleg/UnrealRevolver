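; Player controller that handles movement, look and switching between a main mode and an inspect mode using Enhanced Input.
; It adds the main mapping context on BeginPlay, and a FlipFlop on the switch action swaps it with the inspect context.
; Move input drives the controlled pawn along the controller's right and horizontally flattened forward vectors.
; Aim input applies yaw and pitch scaled by separate horizontal and vertical multipliers.
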(event `self.ReceiveBeginPlay`
  (`EnhancedInputSubsystemInterface.AddMappingContext` (pcsubsystem `EnhancedInputLocalPlayerSubsystem` self) "/Game/Blueprints/Inputs/MainMode/InputContext_MainMode.InputContext_MainMode" 0 (struct)))

(event `EnhancedInput|/Game/Blueprints/Inputs/Input_SwitchModes`
  (params (ActionValue :type Boolean) (ElapsedSeconds :type "Float (double-precision)") (TriggeredSeconds :type "Float (double-precision)") (InputAction :type "InputAction Object Reference" :default "/Game/Blueprints/Inputs/Input_SwitchModes.Input_SwitchModes"))
  (:`Completed`
    (`/Engine/EditorBlueprintResources/StandardMacros.FlipFlop`
      (:`A`
        (`EnhancedInputSubsystemInterface.RemoveMappingContext` (pcsubsystem `EnhancedInputLocalPlayerSubsystem` self) "/Game/Blueprints/Inputs/MainMode/InputContext_MainMode.InputContext_MainMode" (struct))
        (`EnhancedInputSubsystemInterface.AddMappingContext` (pcsubsystem `EnhancedInputLocalPlayerSubsystem` self) "/Game/Blueprints/Inputs/InspectMode/InputContext_InspectMode.InputContext_InspectMode" 0 (struct)))
      (:`B`
        (`EnhancedInputSubsystemInterface.RemoveMappingContext` (pcsubsystem `EnhancedInputLocalPlayerSubsystem` self) "/Game/Blueprints/Inputs/InspectMode/InputContext_InspectMode.InputContext_InspectMode" (struct))
        (`EnhancedInputSubsystemInterface.AddMappingContext` (pcsubsystem `EnhancedInputLocalPlayerSubsystem` self) "/Game/Blueprints/Inputs/MainMode/InputContext_MainMode.InputContext_MainMode" 0 (struct))))))

(event `EnhancedInput|/Game/Blueprints/Inputs/MainMode/Input_Move`
  (params (ActionValue :type "Vector2D Structure") (ElapsedSeconds :type "Float (double-precision)") (TriggeredSeconds :type "Float (double-precision)") (InputAction :type "InputAction Object Reference" :default "/Game/Blueprints/Inputs/MainMode/Input_Move.Input_Move"))
  (bind (_x _y) (`KismetMathLibrary.BreakVector2D` ActionValue))
  (:`Triggered`
    (`Pawn.AddMovementInput` (`self.K2_GetPawn`) (+ (* _x (`self.GetActorRightVector`)) (* _y (`KismetMathLibrary.Normal` (`KismetMathLibrary.MakeVector` (.x (`self.GetActorForwardVector`)) (.y (`self.GetActorForwardVector`)))))) 1.0 false)))

(event `EnhancedInput|/Game/Blueprints/Inputs/MainMode/Input_Aim`
  (params (ActionValue :type "Vector2D Structure") (ElapsedSeconds :type "Float (double-precision)") (TriggeredSeconds :type "Float (double-precision)") (InputAction :type "InputAction Object Reference" :default "/Game/Blueprints/Inputs/MainMode/Input_Aim.Input_Aim"))
  (bind (_x _y) (`KismetMathLibrary.BreakVector2D` ActionValue))
  (:`Triggered`
    (`self.AddYawInput` (* _x (`self.kLookMultiplierHorizontal`)))
    (`self.AddPitchInput` (* _y (`self.kLookMultiplierVertical`)))))

(fn `UserConstructionScript`)