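; Player pawn simulating a hand-operated six-shot revolver with separate inputs for trigger, hammer, safety, cylinder, ejector, loading, aiming and rotation.
; Analog axes pose the parts; the trigger also drives the hammer, which advances the chamber index, and a full pull fires a line trace or dry-fires.
; With the cylinder open, bullets move along splines via the ejector or randomized tilt-based sliding, spawning ejected-bullet actors.
; Custom events play mechanical sounds.
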(event `self.ReceiveBeginPlay`
  (for _ (range 6)
    (`KismetArrayLibrary.Array_Add` (`self.BulletPositions`))
    (`KismetArrayLibrary.Array_Add` (`self.BulletSlidingFactors`))
    (`KismetArrayLibrary.Array_Add` (`self.EjectedBullets`))
    (`KismetArrayLibrary.Array_Add` (`self.SpentBullets`)))
  (`KismetArrayLibrary.Array_Add` (`self.BulletMeshes`) (`self.Bullet0`))
  (`KismetArrayLibrary.Array_Add` (`self.BulletSplines`) (`self.Spline0`))
  (`KismetArrayLibrary.Array_Add` (`self.BulletMeshes`) (`self.Bullet1`))
  (`KismetArrayLibrary.Array_Add` (`self.BulletSplines`) (`self.Spline1`))
  (`KismetArrayLibrary.Array_Add` (`self.BulletMeshes`) (`self.Bullet2`))
  (`KismetArrayLibrary.Array_Add` (`self.BulletSplines`) (`self.Spline2`))
  (`KismetArrayLibrary.Array_Add` (`self.BulletMeshes`) (`self.Bullet3`))
  (`KismetArrayLibrary.Array_Add` (`self.BulletSplines`) (`self.Spline3`))
  (`KismetArrayLibrary.Array_Add` (`self.BulletMeshes`) (`self.Bullet4`))
  (`KismetArrayLibrary.Array_Add` (`self.BulletSplines`) (`self.Spline4`))
  (`KismetArrayLibrary.Array_Add` (`self.BulletMeshes`) (`self.Bullet5`))
  (`KismetArrayLibrary.Array_Add` (`self.BulletSplines`) (`self.Spline5`))
  (`self.PickNewSlidingFactors`))

(event `self.ReceiveTick`
  (params (DeltaSeconds :type "Float (single-precision)"))
  (`self.UpdateBullets`))

(event `EnhancedInput|/Game/Blueprints/Inputs/Input_Trigger`
  (params (ActionValue :type "Float (double-precision)") (ElapsedSeconds :type "Float (double-precision)") (TriggeredSeconds :type "Float (double-precision)") (InputAction :type "InputAction Object Reference" :default "/Game/Blueprints/Inputs/Input_Trigger.Input_Trigger"))
  (:`Triggered`
    (`self.ProcessTrigger` ActionValue :!label _label))
  (:`Completed`
    (goto _label)))

(event `EnhancedInput|/Game/Blueprints/Inputs/Input_SwitchModes`
  (params (ActionValue :type Boolean) (ElapsedSeconds :type "Float (double-precision)") (TriggeredSeconds :type "Float (double-precision)") (InputAction :type "InputAction Object Reference" :default "/Game/Blueprints/Inputs/Input_SwitchModes.Input_SwitchModes"))
  (:`Completed`
    (`/Engine/EditorBlueprintResources/StandardMacros.FlipFlop`
      (:`A`
        (`self.ProcessSwitchModes` true))
      (:`B`
        (`self.ProcessSwitchModes` false)))))

(event `EnhancedInput|/Game/Blueprints/Inputs/MainMode/Input_AimDownSights`
  (params (ActionValue :type Boolean) (ElapsedSeconds :type "Float (double-precision)") (TriggeredSeconds :type "Float (double-precision)") (InputAction :type "InputAction Object Reference" :default "/Game/Blueprints/Inputs/MainMode/Input_AimDownSights.Input_AimDownSights"))
  (:`Completed`
    (bind _isa (`/Engine/EditorBlueprintResources/StandardMacros.FlipFlop`)
      (:`A`
        _)
      (:`B`
        _))
    (`self.ProcessAimDownSights` _isa)))

(event `EnhancedInput|/Game/Blueprints/Inputs/InspectMode/Input_Cylinder`
  (params (ActionValue :type Boolean) (ElapsedSeconds :type "Float (double-precision)") (TriggeredSeconds :type "Float (double-precision)") (InputAction :type "InputAction Object Reference" :default "/Game/Blueprints/Inputs/InspectMode/Input_Cylinder.Input_Cylinder"))
  (:`Completed`
    (bind _isa (`/Engine/EditorBlueprintResources/StandardMacros.FlipFlop`)
      (:`A`
        _)
      (:`B`
        _))
    (`self.ProcessCylinder` _isa)))

(event `EnhancedInput|/Game/Blueprints/Inputs/InspectMode/Input_Ejector`
  (params (ActionValue :type "Float (double-precision)") (ElapsedSeconds :type "Float (double-precision)") (TriggeredSeconds :type "Float (double-precision)") (InputAction :type "InputAction Object Reference" :default "/Game/Blueprints/Inputs/InspectMode/Input_Ejector.Input_Ejector"))
  (:`Triggered`
    (`self.ProcessEjector` ActionValue :!label _label_2))
  (:`Completed`
    (goto _label_2)))

(event `EnhancedInput|/Game/Blueprints/Inputs/InspectMode/Input_Hammer`
  (params (ActionValue :type "Float (double-precision)") (ElapsedSeconds :type "Float (double-precision)") (TriggeredSeconds :type "Float (double-precision)") (InputAction :type "InputAction Object Reference" :default "/Game/Blueprints/Inputs/InspectMode/Input_Hammer.Input_Hammer"))
  (:`Triggered`
    (`self.ProcessHammer` (`KismetMathLibrary.FClamp` ActionValue) :!label _label_3))
  (:`Completed`
    (goto _label_3)))

(event `EnhancedInput|/Game/Blueprints/Inputs/InspectMode/Input_LoadBullet`
  (params (ActionValue :type Boolean) (ElapsedSeconds :type "Float (double-precision)") (TriggeredSeconds :type "Float (double-precision)") (InputAction :type "InputAction Object Reference" :default "/Game/Blueprints/Inputs/InspectMode/Input_LoadBullet.Input_LoadBullet"))
  (:`Completed`
    (`self.ProcessLoadBullet`)))

(event `EnhancedInput|/Game/Blueprints/Inputs/InspectMode/Input_ResetGunOrientation`
  (params (ActionValue :type Boolean) (ElapsedSeconds :type "Float (double-precision)") (TriggeredSeconds :type "Float (double-precision)") (InputAction :type "InputAction Object Reference" :default "/Game/Blueprints/Inputs/InspectMode/Input_ResetGunOrientation.Input_ResetGunOrientation"))
  (:`Completed`
    (`self.ProcessResetGunOrientation`)))

(event `EnhancedInput|/Game/Blueprints/Inputs/InspectMode/Input_Safety`
  (params (ActionValue :type Boolean) (ElapsedSeconds :type "Float (double-precision)") (TriggeredSeconds :type "Float (double-precision)") (InputAction :type "InputAction Object Reference" :default "/Game/Blueprints/Inputs/InspectMode/Input_Safety.Input_Safety"))
  (:`Completed`
    (`self.ProcessSafety` ActionValue)))

(event `EnhancedInput|/Game/Blueprints/Inputs/InspectMode/Input_TurnGun`
  (params (ActionValue :type "Vector2D Structure") (ElapsedSeconds :type "Float (double-precision)") (TriggeredSeconds :type "Float (double-precision)") (InputAction :type "InputAction Object Reference" :default "/Game/Blueprints/Inputs/InspectMode/Input_TurnGun.Input_TurnGun"))
  (bind (_x _y) (`KismetMathLibrary.BreakVector2D` ActionValue))
  (:`Triggered`
    (`self.ProcessTurnGun` _x _y :!label _label_4))
  (:`Completed`
    (goto _label_4)))

(event `OnBarrelCycle`
  (`self.ProcessOnBarrelCycled`))

(event `OnCylinderClosed`
  (`GameplayStatics.PlaySoundAtLocation` "/Game/AudioAssets/CylinderClosed.CylinderClosed" (`SceneComponent.K2_GetComponentLocation` (`self.revolver_body`)) (struct) 1.0 1.0 0.0 null null null null))

(event `OnCylinderOpened`
  (`GameplayStatics.PlaySoundAtLocation` "/Game/AudioAssets/CylinderOpen.CylinderOpen" (`SceneComponent.K2_GetComponentLocation` (`self.revolver_body`)) (struct) 1.0 1.0 0.0 null null null null))

(event `OnDryFire`
  (`GameplayStatics.PlaySoundAtLocation` "/Game/AudioAssets/dryFire.DryFire" (`SceneComponent.K2_GetComponentLocation` (`self.revolver_body`)) (struct) 1.0 1.0 0.0 null null null null))

(event `OnEjectorPushed`
  (`GameplayStatics.PlaySoundAtLocation` "/Game/AudioAssets/EjectorOn.EjectorOn" (`SceneComponent.K2_GetComponentLocation` (`self.revolver_body`)) (struct) 1.0 1.0 0.0 null null null null))

(event `OnEjectorReleased`
  (`GameplayStatics.PlaySoundAtLocation` "/Game/AudioAssets/EjectorOff.EjectorOff" (`SceneComponent.K2_GetComponentLocation` (`self.revolver_body`)) (struct) 1.0 1.0 0.0 null null null null))

(event `OnFullyCocked`
  (`GameplayStatics.PlaySoundAtLocation` "/Game/AudioAssets/FullCocking.FullCocking" (`SceneComponent.K2_GetComponentLocation` (`self.revolver_body`)) (struct) 1.0 1.0 0.0 null null null null))

(event `OnBulletInserted`
  (`GameplayStatics.PlaySoundAtLocation` "/Game/AudioAssets/InsertedBullet.InsertedBullet" (`SceneComponent.K2_GetComponentLocation` (`self.revolver_body`)) (struct) 1.0 1.0 0.0 null null null null))

(event `OnSafetyOn`
  (`GameplayStatics.PlaySoundAtLocation` "/Game/AudioAssets/SafetyOn.SafetyOn" (`SceneComponent.K2_GetComponentLocation` (`self.revolver_body`)) (struct) 1.0 1.0 0.0 null null null null))

(event `OnSafetyOff`
  (`GameplayStatics.PlaySoundAtLocation` "/Game/AudioAssets/SafetyOff.SafetyOff" (`SceneComponent.K2_GetComponentLocation` (`self.revolver_body`)) (struct) 1.0 1.0 0.0 null null null null))

(event `OnTriggerReleasedWithoutFiring`
  (`GameplayStatics.PlaySoundAtLocation` "/Game/AudioAssets/TriggerRelease.TriggerRelease" (`SceneComponent.K2_GetComponentLocation` (`self.revolver_body`)) (struct) 1.0 1.0 0.0 null null null null))

(event `OnGunFired`
  (`GameplayStatics.PlaySoundAtLocation` "/Game/AudioAssets/bang.bang" (`SceneComponent.K2_GetComponentLocation` (`self.revolver_body`)) (struct) 1.0 1.0 0.0 null null null null))

(fn `FireGun`
  (bind _returnvalue (`SceneComponent.K2_GetComponentLocation` (`self.revolver_body`)))
  (bind _output_get (set `self.HammerAxis` 0.0))
  (`self.ProcessHammer` _output_get)
  (set `self.Fired` true)
  (if (not (`|GetArrayItem` (`self.SpentBullets`) (`self.CurrentBullet`)))
    (`KismetArrayLibrary.Array_Set` (`self.SpentBullets`) (`self.CurrentBullet`) true)
    (`self.OnGunFired`)
    (bind _outhit (`KismetSystemLibrary.LineTraceSingle` :`Start` _returnvalue :`End` (+ _returnvalue (* (`SceneComponent.GetForwardVector` (`self.revolver_body`)) 10000.0)) :`TraceChannel` "TraceTypeQuery1" :`DrawDebugType` "ForOneFrame"))
    (bind (_bblockinghit _binitialoverlap _time _distance _location) (`GameplayStatics.BreakHitResult` _outhit))
    (if _bblockinghit
      (`|SpawnActorFromClass` "/Game/Blueprints/Gun/HitParticles.HitParticles_C" (`KismetMathLibrary.Conv_VectorToTransform` _location) "AlwaysSpawn" "OverrideRootScale" null null))
    (else
      (`self.OnDryFire`))))

(fn `PickNewSlidingFactors`
  (for (_ _array_index) (`self.BulletSlidingFactors`)
    (`KismetArrayLibrary.Array_Set` (`self.BulletSlidingFactors`) _array_index (`KismetMathLibrary.RandomFloatInRange` (`self.kBulletSlidingFactorRangeMin_`) (`self.kBulletSlidingFactorRangeMax_`)))))

(fn `ProcessAimDownSights`
  (params (AimDownSights :type Boolean))
  (if (`local.AimDownSights`)
    (`SceneComponent.K2_AddRelativeLocation` (`self.revolver_body`) (0.0 -20.0 5.0) false true)
    (else
      (`SceneComponent.K2_AddRelativeLocation` (`self.revolver_body`) (0.0 20.0 -5.0) false true))))

(fn `ProcessCylinder`
  (params (IsOpen :type Boolean))
  (if (`KismetMathLibrary.NearlyEqual_FloatFloat` (`self.HammerAxis`) 0.0 0.05)
    (set `self.CurrentBullet` 0)
    (bind _output_get (set `self.CylinderIsOpen` (`local.IsOpen`)))
    (`self.SetCylinderPosition` _output_get)))

(fn `ProcessEjector`
  (params (EjectionAxis :type "Float (double-precision)"))
  (if (`self.CylinderIsOpen`)
    (bind _output_get (set `self.EjectorAxis` (`local.EjectionAxis`)))
    (`self.SetEjectorPosition` _output_get)
    (else
      (`self.SetEjectorPosition` 0.0))))

(fn `ProcessHammer`
  (params (CockingAxis :type "Float (double-precision)"))
  (locals (lastAxis :type "Float (double-precision)"))
  (if (and (not (`self.SafetyIsOn`)) (not (`KismetMathLibrary.NearlyEqual_FloatFloat` (`self.HammerAxis`) 1.0 0.05)))
    (set `local.lastAxis` (`self.HammerAxis`))
    (bind _output_get (set `self.HammerAxis` (`local.CockingAxis`)))
    (`self.SetHammerRotation` _output_get)
    (if (and (< (`local.lastAxis`) (`self.HammerAxis`)) (> (`self.HammerAxis`) 0.95))
      (`self.OnFullyCocked`))
    (if (and (> (`local.lastAxis`) (`self.HammerAxis`)) (< (`self.HammerAxis`) 0.05) (> (`KismetMathLibrary.Abs` (- (`local.lastAxis`) (`self.HammerAxis`))) (`self.kDryFireThreshold_`)))
      (`self.OnDryFire`))
    (if (and (> (`self.HammerAxis`) (`local.lastAxis`)) (> (`self.HammerAxis`) 0.5) (< (`local.lastAxis`) 0.5))
      (`self.OnBarrelCycle`))))

(fn `ProcessLoadBullet`
  (if (`self.CylinderIsOpen`)
    (bind _result (`/Engine/EditorBlueprintResources/StandardMacros.IncrementInt` (`self.CurrentBullet`))
      (:`  `
        (set `self.CurrentBullet` (mod _result 6))
        (if (`|GetArrayItem` (`self.EjectedBullets`) (`self.CurrentBullet`))
          (`KismetArrayLibrary.Array_Set` (`self.EjectedBullets`) (`self.CurrentBullet`))
          (`SceneComponent.SetVisibility` (`|GetArrayItem` (`self.BulletMeshes`) (`self.CurrentBullet`)) true false)
          (`KismetArrayLibrary.Array_Set` (`self.BulletPositions`) (`self.CurrentBullet`))
          (`KismetArrayLibrary.Array_Set` (`self.SpentBullets`) (`self.CurrentBullet`))
          (`self.OnBulletInserted`))))))

(fn `ProcessOnBarrelCycled`
  (locals (lastAxis :type "Float (double-precision)"))
  (`GameplayStatics.PlaySoundAtLocation` "/Game/AudioAssets/BarrelCycle.BarrelCycle" (`SceneComponent.K2_GetComponentLocation` (`self.revolver_body`)) (struct) 1.0 1.0 0.0 null null null null)
  (bind _result (`/Engine/EditorBlueprintResources/StandardMacros.IncrementInt` (`self.CurrentBullet`))
    (:`  `
      (set `self.CurrentBullet` (mod _result 6)))))

(fn `ProcessResetGunOrientation`
  (`SceneComponent.K2_SetRelativeRotation` (`self.revolver_body`) (struct :`Pitch` 25.0 :`Yaw` -45.0) false false))

(fn `ProcessSafety`
  (params (SafetyOn :type Boolean))
  (if (`KismetMathLibrary.NearlyEqual_FloatFloat` (`self.HammerAxis`) 0.0 0.05)
    (bind _output_get (set `self.SafetyIsOn` (`local.SafetyOn`)))
    (`self.SetSafetyPosition` _output_get)))

(fn `ProcessSwitchModes`
  (params (InspectModeOn :type Boolean))
  (if (`local.InspectModeOn`)
    (`SceneComponent.K2_AddRelativeLocation` (`self.revolver_body`) (0.0 -20.0 5.0) false true)
    (`SceneComponent.K2_AddRelativeRotation` (`self.revolver_body`) (struct :`Pitch` 25.0 :`Yaw` -45.0) false true)
    (else
      (`SceneComponent.K2_AddRelativeLocation` (`self.revolver_body`) (0.0 20.0 -5.0) false true)
      (`SceneComponent.K2_AddRelativeRotation` (`self.revolver_body`) (struct :`Pitch` -25.0 :`Yaw` 45.0) false true))))

(fn `ProcessTrigger`
  (params (PullingAxis :type "Float (double-precision)"))
  (locals (lastAxis :type "Float (double-precision)"))
  (if (not (`self.SafetyIsOn`))
    (set `local.lastAxis` (`self.TriggerAxis`))
    (bind _output_get (set `self.TriggerAxis` (`local.PullingAxis`)))
    (`self.SetTriggerRotation` _output_get)
    (if (not (`self.Fired`))
      (`self.ProcessHammer` (`self.TriggerAxis`)))
    (if (and (> (`local.lastAxis`) (`self.TriggerAxis`)) (`KismetMathLibrary.NearlyEqual_FloatFloat` (`self.TriggerAxis`) 0.0 0.05))
      (`self.OnTriggerReleasedWithoutFiring`))
    (if (and (`self.Fired`) (< (`self.TriggerAxis`) 0.45))
      (set `self.Fired` false))
    (if (and (not (`self.Fired`)) (`KismetMathLibrary.NearlyEqual_FloatFloat` (`self.TriggerAxis`) 1.0 0.05))
      (`self.FireGun`))))

(fn `ProcessTurnGun`
  (params (X :type "Float (double-precision)") (Y :type "Float (double-precision)"))
  (`SceneComponent.K2_AddRelativeRotation` (`self.revolver_body`) (`KismetMathLibrary.MakeRotator` 0.0 (`local.Y`) (`local.X`)) false false))

(fn `SetBulletPosition`
  (params (Idx :type Integer))
  (`SceneComponent.K2_SetRelativeLocation` (`|GetArrayItem` (`self.BulletMeshes`) (`local.Idx`)) (`SplineComponent.GetLocationAtTime` (`|GetArrayItem` (`self.BulletSplines`) (`local.Idx`)) (`|GetArrayItem` (`self.BulletPositions`) (`local.Idx`)) "Local" false) false true))

(fn `SetCylinderCoaxialRotation`
  (params (Idx :type Integer))
  (locals (Value :type "Float (double-precision)"))
  (`SceneComponent.K2_SetRelativeRotation` (`self.revolver_cylinder`) (`KismetMathLibrary.MakeRotator` (* Idx 60.0)) false false))

(fn `SetCylinderPosition`
  (params (OpenOrClosed :type Boolean))
  (if OpenOrClosed
    (`SceneComponent.K2_SetRelativeLocation` (`self.revolver_cylinder`) (`KismetMathLibrary.MakeVector` (.x (`SceneComponent.RelativeLocation` (`self.revolver_cylinder`))) (- 0.0 (.z (`SceneComponent.RelativeLocation` (`self.revolver_cylinder`)))) (.y (`SceneComponent.RelativeLocation` (`self.revolver_cylinder`)))) false true)
    (else
      (`SceneComponent.K2_SetRelativeLocation` (`self.revolver_cylinder`) (`KismetMathLibrary.MakeVector` (.x (`SceneComponent.RelativeLocation` (`self.revolver_cylinder`))) (.z (`SceneComponent.RelativeLocation` (`self.revolver_cylinder`))) (- 0.0 (.y (`SceneComponent.RelativeLocation` (`self.revolver_cylinder`))))) false true))))

(fn `SetEjectorPosition`
  (params (Percentage :type "Float (double-precision)"))
  (`SceneComponent.K2_SetRelativeLocation` (`self.revolver_ejector`) (`KismetMathLibrary.VLerp` (-37.0 0.0 0.0) (-47.0 0.0 0.0) Percentage) false true))

(fn `SetHammerRotation`
  (params (Percentage :type "Float (double-precision)"))
  (`SceneComponent.K2_SetRelativeRotation` (`self.revolver_hammer`) (`KismetMathLibrary.MakeRotator` 0.0 (* Percentage 65.0)) false true))

(fn `SetSafetyPosition`
  (params (OnOrOff :type Boolean))
  (locals (Value :type "Float (double-precision)"))
  (if OnOrOff
    (`SceneComponent.K2_AddRelativeLocation` (`self.revolver_safety`) (-10.0 0.0 0.0) false true)
    (else
      (`SceneComponent.K2_AddRelativeLocation` (`self.revolver_safety`) (10.0 0.0 0.0) false true))))

(fn `SetTriggerRotation`
  (params (Percentage :type "Float (double-precision)"))
  (`SceneComponent.K2_SetRelativeRotation` (`self.revolver_trigger`) (`KismetMathLibrary.MakeRotator` 0.0 (* Percentage -54.0)) false false))

(fn `UpdateBullets`
  (if (`self.CylinderIsOpen`)
    (for (_ _array_index) (`self.BulletPositions`)
      (`self.UpdateSingleBullet` _array_index))
    (else
      (for (_ _array_index_2) (`self.BulletPositions`)
        (`KismetArrayLibrary.Array_Set` (`self.BulletPositions`) _array_index_2)
        (`self.SetBulletPosition` _array_index_2)))))

(fn `UpdateSingleBullet`
  (params (Idx :type Integer))
  (if (<= (`|GetArrayItem` (`self.BulletPositions`) (`local.Idx`)) (* (`self.EjectorAxis`) (`self.kBulletEjectionOffset_`)))
    (`KismetArrayLibrary.Array_Set` (`self.BulletPositions`) (`local.Idx`) (`KismetMathLibrary.FClamp` (* (`self.EjectorAxis`) (`self.kBulletEjectionOffset_`))))
    (elif (> (`KismetMathLibrary.Abs` (* (`self.ComputeDotBetweenFrontAndUp`) (`|GetArrayItem` (`self.BulletSlidingFactors`) (`local.Idx`)))) (`self.kBulletSlidingThreshold_`))
      (`KismetArrayLibrary.Array_Set` (`self.BulletPositions`) (`local.Idx`) (`KismetMathLibrary.FClamp` (+ (`|GetArrayItem` (`self.BulletPositions`) (`local.Idx`)) (* (`self.ComputeDotBetweenFrontAndUp`) (`|GetArrayItem` (`self.BulletSlidingFactors`) (`local.Idx`))))))))
  (if (and (not (`|GetArrayItem` (`self.EjectedBullets`) (`local.Idx`))) (`KismetMathLibrary.NearlyEqual_FloatFloat` (`|GetArrayItem` (`self.BulletPositions`) (`local.Idx`)) 1.0 0.075))
    (`SceneComponent.SetVisibility` (`|GetArrayItem` (`self.BulletMeshes`) (`local.Idx`)) false false)
    (`|SpawnActorFromClass` "/Game/Blueprints/Gun/EjectedBullet.EjectedBullet_C" (`SceneComponent.K2_GetComponentToWorld` (`|GetArrayItem` (`self.BulletMeshes`) (`local.Idx`))) "AdjustIfPossibleButAlwaysSpawn" "OverrideRootScale" null null)
    (`KismetArrayLibrary.Array_Set` (`self.EjectedBullets`) (`local.Idx`) true))
  (`self.SetBulletPosition` (`local.Idx`)))

(fn `UserConstructionScript`)